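; Moving floor actor that travels up and down in a repeating cycle, pausing at each end.
; A BeginPlay delay loop drives the MoveState enum: three seconds of travel, a two-second stop, then the opposite direction.
; Tick reads that state and offsets the actor along local Z at a constant, delta-time-scaled speed without sweep.
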(event `self.ReceiveBeginPlay`
  (`KismetSystemLibrary.Delay` 3.0 :!label _label)
  (switch `/Game/ActiveRoom/Enum/EMovementFloorState` (`self.MoveState`)
    (:`NewEnumerator1`
      (set `self.MoveState` "NewEnumerator0")
      (`KismetSystemLibrary.Delay` 2.0)
      (set `self.MoveState` "NewEnumerator2")
      (goto _label))
    (:`NewEnumerator2`
      (set `self.MoveState` "NewEnumerator0")
      (`KismetSystemLibrary.Delay` 2.0)
      (set `self.MoveState` "NewEnumerator1")
      (goto _label))))

(event `self.ReceiveTick`
  (params (DeltaSeconds :type "Float (single-precision)"))
  (bind _returnvalue (* DeltaSeconds 100.0))
  (switch `/Game/ActiveRoom/Enum/EMovementFloorState` (`self.MoveState`)
    (:`NewEnumerator1`
      (`self.K2_AddActorLocalOffset` (`KismetMathLibrary.MakeVector` 0.0 0.0 _returnvalue)))
    (:`NewEnumerator2`
      (`self.K2_AddActorLocalOffset` (`KismetMathLibrary.MakeVector` 0.0 0.0 (* _returnvalue -1.0))))))

(fn `UserConstructionScript`)